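; Ammo pickup item that grants the first-person player extra munitions when collected.
; On collision, it casts to FirstPersonCharacter and adds a fixed amount to its Minutions counter.
; It then spawns a Niagara coin-shower effect at the player, notifies the game mode through RemoveOneItemMessage, and destroys itself.
; The construction script only runs the parent's, so setup and collision detection come from a parent class.
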(event EventOnCollision
  (params (Player :type First%20Person%20Character%20Object%20Reference))
  (bind _asfirst_person_character (Utilities|Casting|CastToFirstPersonCharacter Player))
  (Variables|/Game/FirstPersonBP/Blueprints/FirstPersonCharacter.FirstPersonCharacter_C|Setminutions _asfirst_person_character (+ (Variables|/Game/FirstPersonBP/Blueprints/FirstPersonCharacter.FirstPersonCharacter_C|Getminutions _asfirst_person_character) 60))
  (Niagara|SpawnSystematLocation "/Game/sA_PickupSet_1/Fx/NiagaraSystems/NS_Coin_Shower.NS_Coin_Shower" (Transformation|GetActorLocation Player) "0, 0, 0" "1.500000,1.500000,1.500000")
  (Class|BPIGameModeMP|RemoveOneItem(Message) (Game|GetGameMode))
  (Actor|DestroyActor))

(fn ConstructionScript
  (|CallParentFunction))