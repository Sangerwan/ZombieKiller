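; BP_Spawn is a zombie spawner that creates BP_NPC enemies inside a spawn zone volume.
; On BeginPlay it registers itself with the game mode through a message call.
; SpawnOneEnnemy asks the game mode for permission, spawns the AI at a random point in ZombieSpawnZone, then notifies the game mode of the added enemy.
; The random point uses the scaled box extent, so resizing the zone is respected.
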(event Custom|SpawnOneEnnemy
  (bind _zombie_spawn_zone (Variables|Default|Getzombie_spawn_zone))
  ;[1 1 1] Take a random position and summon a zombie
  (bind _can (Class|BPIGameModeMP|CanSpawnOneEnnemy(Message) (Game|GetGameMode)))
  (if _can
    (AI|SpawnAIFromClass "/Game/FirstPersonBP/Blueprints/IA/BP_NPC.BP_NPC_C" 0 (Math|Random|RandomPointinBoundingBox (Transformation|GetWorldLocation _zombie_spawn_zone) (Components|Box|GetScaledBoxExtent _zombie_spawn_zone)) "0, 0, 0" false 0)
    (Class|BPIGameModeMP|AddOneEnnemy(Message) (Game|GetGameMode))))

(event EventBeginPlay
  ;[1 1 1] envoi ref au game mode
  (Class|BPIGameModeMP|RegisterSpawner(Message) (Game|GetGameMode) self))

(fn ConstructionScript)