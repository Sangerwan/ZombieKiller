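; Spawner Blueprint that keeps a capped population of BPItem actors inside its SpawnZone volume.
; Its Spawn override calls the parent and SpawnEvent only while ItemCount is below MaxItemCount; SpawnEvent places an item at a random point in the zone.
; Each item's OnDestroyed event lowers ItemCount after a single shared SpawnRate Delay, so destructions during a pending delay are not counted separately.
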(event Custom|SpawnEvent
  (bind _spawn_zone (Variables|Default|Getspawn_zone))
  (bind _returnvalue (Game|SpawnActorfromClass (Variables|Default|GetBP_Item) (Math|Conversions|ToTransform(Vector) (Math|Random|RandomPointinBoundingBox (Transformation|GetWorldLocation _spawn_zone) (Components|Box|GetScaledBoxExtent _spawn_zone))) "AdjustIfPossibleButAlwaysSpawn" 0 0))
  (if (Utilities|IsValid _returnvalue)
    (Game|BindEventtoOnDestroyed _returnvalue (delegate Custom|OnItemDestroy))
    (Variables|Default|SetItemCount (+ (Variables|Default|GetItemCount) 1))))

(event Custom|OnItemDestroy
  (params (DestroyedActor :type Actor%20Object%20Reference))
  (Utilities|FlowControl|Delay (Variables|Default|GetSpawnRate))
  (Variables|Default|SetItemCount (- (Variables|Default|GetItemCount) 1)))

(event EventBeginPlay
  (|CallParentFunction))

(fn ConstructionScript)

(fn Spawn
  (if (< (Variables|Default|GetItemCount) (Variables|Default|GetMaxItemCount))
    (|CallParentFunction)
    (CallFunction|SpawnEvent)))