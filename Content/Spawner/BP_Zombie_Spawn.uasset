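; Zombie spawner that creates BP_NPC actors at random points inside its SpawnZone box.
; Spawn proceeds only while both the game mode's zombie count and this spawner's own count are below their maximums, calling the parent Spawn first.
; Each spawned NPC's OnDestroyed is bound to a handler that waits SpawnRate before decrementing the local count, delaying when that slot frees up.
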(event Custom|SpawnEvent
  (bind _spawn_zone (Variables|Default|Getspawn_zone))
  (bind _returnvalue (Game|SpawnActorfromClass "/Game/Zombie/IA/BP_NPC.BP_NPC_C" (Math|Conversions|ToTransform(Vector) (Math|Random|RandomPointinBoundingBox (Transformation|GetWorldLocation _spawn_zone) (Components|Box|GetScaledBoxExtent _spawn_zone))) "AdjustIfPossibleButAlwaysSpawn" 0 0))
  (Game|BindEventtoOnDestroyed _returnvalue (delegate Custom|OnZombieDestroy))
  (Variables|Default|SetZombieCount (+ (Variables|Default|GetZombieCount) 1)))

(event Custom|OnZombieDestroy
  (params (DestroyedActor :type Actor%20Object%20Reference))
  (Utilities|FlowControl|Delay (Variables|Default|GetSpawnRate))
  (Variables|Default|SetZombieCount (- (Variables|Default|GetZombieCount) 1)))

(event EventBeginPlay
  ;[1 1 1] envoi ref au game mode
  (|CallParentFunction))

(fn ConstructionScript)

(fn Spawn
  (bind _asfirst_person_game_mode (Utilities|Casting|CastToFirstPersonGameMode (Game|GetGameMode)))
  (if (< (Variables|/Game/FirstPersonBP/Blueprints/FirstPersonGameMode.FirstPersonGameMode_C|GetZombieCount _asfirst_person_game_mode) (Variables|/Game/FirstPersonBP/Blueprints/FirstPersonGameMode.FirstPersonGameMode_C|GetMaxZombieCount _asfirst_person_game_mode))
    (if (< (Variables|Default|GetZombieCount) (Variables|Default|GetMaxZombieCount))
      (|CallParentFunction)
      (CallFunction|SpawnEvent))))