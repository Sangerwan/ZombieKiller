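; AI controller for zombie NPCs that runs the BT_NPC behavior tree when it possesses a pawn.
; Perception updates for actors tagged Player write a sight flag to the blackboard.
; The same updates switch the NPC's walk speed between a faster chase pace and a slow default.
; The controlled NPC reference is supplied through the SetNPC function.
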(event OnTargetPerceptionUpdated(AIPerception)
  (params (Actor :type Actor%20Object%20Reference) (Stimulus :type AI%20Stimulus%20Structure))
  (bind _bsuccessfullysensed (Utilities|Struct|BreakAIStimulus Stimulus))
  (bind _bp_npc (Variables|Default|GetBP_NPC))
  (bind _charactermovement (Variables|/Script/Engine.Character|GetCharacterMovement _bp_npc))
  (if (Actor|ActorHasTag Actor "Player")
    (AI|Components|Blackboard|SetValueasBool (Variables|Default|GetBlackboard) (Variables|Default|GetBB_Key_isPlayerInsight) _bsuccessfullysensed)
    (if _bsuccessfullysensed
      (Variables|/Script/Engine.CharacterMovementComponent|SetMaxWalkSpeed _charactermovement 175.0)
      (else
        (Variables|/Script/Engine.CharacterMovementComponent|SetMaxWalkSpeed _charactermovement 75.0)))))

(event EventPossess
  (params (PossessedPawn :type Pawn%20Object%20Reference))
  (AI|RunBehaviorTree "/Game/Zombie/IA/BT_NPC.BT_NPC"))

(fn ConstructionScript)

(fn SetNPC
  (params (NewParam :type BP%20NPC%20Object%20Reference))
  (Variables|Default|SetBP_NPC NewParam))