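; Zombie enemy NPC with health that damages the player on contact and adds to the player's score on death.
; On BeginPlay it binds itself to its health bar widget and registers with BP_NPC_Controller.
; A sphere overlap shows or hides the health bar, while capsule overlap runs a looping timer that sends damage through a health interface message.
; Health interface events clamp health and destroy the actor at zero; IsMaxHealth always returns false.
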(event OnComponentBeginOverlap(Sphere)
  (params (OverlappedComponent :type Primitive%20Component%20Object%20Reference) (OtherActor :type Actor%20Object%20Reference) (OtherComp :type Primitive%20Component%20Object%20Reference) (OtherBodyIndex :type Integer) (bFromSweep :type Boolean) (SweepResult :type Hit%20Result%20Structure%20%28by%20ref%29))
  (Utilities|Casting|CastToFirstPersonCharacter OtherActor)
  (Rendering|SetVisibility (Variables|Default|GetWidget) true false))

(event OnComponentEndOverlap(Sphere)
  (params (OverlappedComponent :type Primitive%20Component%20Object%20Reference) (OtherActor :type Actor%20Object%20Reference) (OtherComp :type Primitive%20Component%20Object%20Reference) (OtherBodyIndex :type Integer))
  (Utilities|Casting|CastToFirstPersonCharacter OtherActor)
  (Rendering|SetVisibility (Variables|Default|GetWidget) false false))

(event OnComponentBeginOverlap(CapsuleComponent)
  (params (OverlappedComponent :type Primitive%20Component%20Object%20Reference) (OtherActor :type Actor%20Object%20Reference) (OtherComp :type Primitive%20Component%20Object%20Reference) (OtherBodyIndex :type Integer) (bFromSweep :type Boolean) (SweepResult :type Hit%20Result%20Structure%20%28by%20ref%29))
  (if (== OtherActor (Game|GetPlayerCharacter 0))
    (Variables|Default|SetOverlappingPlayer? true)
    (CallFunction|ApplyDamage)
    (Utilities|Time|SetTimerbyFunctionName 0 "ApplyDamage" (Variables|Default|GetDamageTickRate) true)))

(event OnComponentEndOverlap(CapsuleComponent)
  (params (OverlappedComponent :type Primitive%20Component%20Object%20Reference) (OtherActor :type Actor%20Object%20Reference) (OtherComp :type Primitive%20Component%20Object%20Reference) (OtherBodyIndex :type Integer))
  (if (== OtherActor (Game|GetPlayerCharacter 0))
    (Variables|Default|SetOverlappingPlayer? false)
    (Utilities|Time|ClearTimerbyFunctionName 0 "ApplyDamage")))

(event Custom|ApplyDamage
  (if (Variables|Default|GetOverlappingPlayer?)
    (Class|IHeath|DecreaseHealth(Message) (Game|GetPlayerCharacter 0) (Variables|Default|GetDamage))))

(event EventBeginPlay
  (bind _asui_enemy_health_bar (Utilities|Casting|CastToUI_EnemyHealthBar (UserInterface|GetUserWidgetObject (Variables|Default|GetWidget))))
  (Variables|/Game/UI/UI_EnemyHealthBar.UI_EnemyHealthBar_C|SetActorRef _asui_enemy_health_bar self)
  (bind _asbp_npc_controller (Utilities|Casting|CastToBP_NPC_Controller (Pawn|GetController)))
  (Default|SetNPC _asbp_npc_controller self))

(event Collision|EventActorBeginOverlap
  (params (OtherActor :type Actor%20Object%20Reference)))

(event EventTick
  (params (DeltaSeconds :type Float%20%28single-precision%29)))

(event EventIncreaseHealth
  (params (Health :type Float%20%28single-precision%29))
  ;[1 1 1] I_Health
  (Variables|Default|SetCurrent%20Health (Math|Float|Min(Float) (Variables|Default|GetMax%20Health) (+ Health (Variables|Default|GetCurrent%20Health)))))

(event EventDecreaseHealth
  (params (Health :type Float%20%28single-precision%29))
  ;[1 1 1] I_Health
  (bind _output_get (Variables|Default|SetCurrent%20Health (Math|Float|Max(Float) (- (Variables|Default|GetCurrent%20Health) Health) 0.0)))
  (if (<= _output_get 0.0)
    (CallFunction|OnDeath)))

(event EventOnDeath
  ;[1 1 1] I_Health
  (bind _asfirst_person_character (Utilities|Casting|CastToFirstPersonCharacter (Game|GetPlayerCharacter 0)))
  (Math|Integer|IncrementInt (Variables|/Game/FirstPersonBP/Blueprints/FirstPersonCharacter.FirstPersonCharacter_C|GetScore _asfirst_person_character)
    (:%20%20
      (Actor|DestroyActor))))

(fn ConstructionScript)

(fn GetCurrentHealth
  (return (Variables|Default|GetCurrent%20Health)))

(fn GetMaxHealth
  (return (Variables|Default|GetMax%20Health)))

(fn IsMaxHealth
  (return false))